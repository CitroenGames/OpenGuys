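; BP_Character is a player character built on ALS (Advanced Locomotion System) that sets up animation layers and chooses mantling settings.
; On BeginPlay it links the default ALS anim class layers to the mesh.
; SelectMantlingSettings uses the high settings for high and in-air mantles.
; For low mantles it switches on the overlay mode gameplay tag to pick default, left, right, both-hands or box variants to suit the held item or state.
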(event EventBeginPlay
  (Components|SkeletalMesh|AnimationBlueprintLinking|LinkAnimClassLayers (Variables|Character|GetMesh) "/ALS/ALS/Character/AnimationInstances/Overlays/AB_Als_Default.AB_Als_Default_C"))

(fn ConstructionScript)

(fn SelectMantlingSettings
  (params (MantlingType :type EAlsMantlingType%20Enum :default "High"))
  (switch Utilities|FlowControl|Switch|SwitchonEAlsMantlingType MantlingType
    (:High
      _)
    (:Low
      (|SwitchGameplayTag (Variables|Default|GetOverlayMode)
        (:Default
          (return "/ALS/ALS/Data/Character/Mantle/MS_Als_Low.MS_Als_Low"))
        (:Als.OverlayMode.Injured
          _)
        (:Als.OverlayMode.HandsTied
          (return "/ALS/ALS/Data/Character/Mantle/MS_Als_Low_BothHands.MS_Als_Low_BothHands"))
        (:Als.OverlayMode.M4
          (return "/ALS/ALS/Data/Character/Mantle/MS_Als_Low_Right.MS_Als_Low_Right"))
        (:Als.OverlayMode.PistolOneHanded
          (return "/ALS/ALS/Data/Character/Mantle/MS_Als_Low_Right.MS_Als_Low_Right"))
        (:Als.OverlayMode.PistolTwoHanded
          (return "/ALS/ALS/Data/Character/Mantle/MS_Als_Low_Right.MS_Als_Low_Right"))
        (:Als.OverlayMode.Bow
          _)
        (:Als.OverlayMode.Torch
          _)
        (:Als.OverlayMode.Binoculars
          (return "/ALS/ALS/Data/Character/Mantle/MS_Als_Low_Right.MS_Als_Low_Right"))
        (:Als.OverlayMode.Box
          (return "/ALS/ALS/Data/Character/Mantle/MS_Als_Low_Box.MS_Als_Low_Box"))
        (:Als.OverlayMode.Barrel
          _))
      (return "/ALS/ALS/Data/Character/Mantle/MS_Als_Low_Left.MS_Als_Low_Left"))
    (:InAir
      _))
  (return "/ALS/ALS/Data/Character/Mantle/MS_Als_High.MS_Als_High"))
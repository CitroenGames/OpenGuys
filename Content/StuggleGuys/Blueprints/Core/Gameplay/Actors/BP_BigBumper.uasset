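; Big bumper obstacle that slides back and forth after random delays and reports hits to the characters it touches.
; On the server, a looping timeline moves the bumper mesh along local Y after each random wait.
; A separate collision box steps along Y on fixed delays tuned to the timeline, and recenters between runs to avoid hits.
; Server-side box overlaps call OnPlayerCollision on the CG_BaseCharacter.
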(event OnComponentBeginOverlap(Box)
  (params (OverlappedComponent :type Primitive%20Component%20Object%20Reference) (OtherActor :type Actor%20Object%20Reference) (OtherComp :type Primitive%20Component%20Object%20Reference) (OtherBodyIndex :type Integer) (bFromSweep :type Boolean) (SweepResult :type Hit%20Result%20Structure%20%28by%20ref%29))
  ;[0.05098 0.05098 0.05098] Forwards the Collided event to the Character that was hit
  (Networking|SwitchHasAuthority
    (:Authority
      (bind _ascg_base_character (Utilities|Casting|CastToCG_BaseCharacter OtherActor))
      (Class|CGPlayerInterface|OnPlayerCollision _ascg_base_character self))))

(event Custom|Set_CollisionVolume
  ;[0.05098 0.05098 0.05098] Moves the collision volume forward and backwards based on a delay which aims for the bumper movement times from the timeline
  (Transformation|SetRelativeLocation (Variables|Default|GetBox) "0.000000,20.000000,200.000000" false false)
  (Utilities|FlowControl|Delay 0.3) ; Between 0 - 0.3 seconds the\nbumper moves forward
  (Transformation|SetRelativeLocation (Variables|Default|GetBox) "0,0.000000,200.000000" false false)
  (Utilities|FlowControl|Delay 0.7) ; Between 1 - 2 seconds the\nbumper moves forward
  (Transformation|SetRelativeLocation (Variables|Default|GetBox) "0,-20.000000,200.000000" false false))

(event EventBeginPlay
  (Networking|SwitchHasAuthority :!label _label
    (:Authority
      ;[0.05098 0.05098 0.05098] Resets x and y location to 0 so the collision volume can't hit a player
      (Transformation|SetRelativeLocation (Variables|Default|GetBox) "0, 0,200.000000" false false)
      ;[0.05098 0.05098 0.05098 1 16] Randomly call Move_Bumper
      (Utilities|FlowControl|Delay (Math|Random|RandomFloatinRange 1.0 3.0))
      ;[0.05098 0.05098 0.05098] Calls SetCollisionVolume, and moves the bumper
      (CallFunction|SetCollisionVolume)
      (bind _location (Timeline|Move_Bumper PlayFromStart)
        (:Update
          (Transformation|SetRelativeLocation (Variables|Default|GetSM_BigBumper) (Math|Vector|MakeVector 0.0 _location 0.0) false false))
        (:Finished
          (goto _label))))))

(fn ConstructionScript)